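; BP_Door_Type7 is a swinging door that the player opens and closes with F from either of two trigger boxes.
; Each box sets its own flag and toggles input, with a short delay on entry, to select a +90 or -90 degree swing.
; FlipFlops play or reverse that side's rotation timeline.
; When the door's world yaw fails that side's closed-or-open check, F reverses the opposite timeline instead.
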(event OnComponentBeginOverlap(90DegreesBox)
  (params (OverlappedComponent :type Primitive%20Component%20Object%20Reference) (OtherActor :type Actor%20Object%20Reference) (OtherComp :type Primitive%20Component%20Object%20Reference) (OtherBodyIndex :type Integer) (bFromSweep :type Boolean) (SweepResult :type Hit%20Result%20Structure%20%28by%20ref%29))
  (Utilities|FlowControl|Delay 0.2)
  (Variables|Default|SetisIn90Box true)
  (Input|EnableInput (Game|GetPlayerController 0)))

(event OnComponentEndOverlap(90DegreesBox)
  (params (OverlappedComponent :type Primitive%20Component%20Object%20Reference) (OtherActor :type Actor%20Object%20Reference) (OtherComp :type Primitive%20Component%20Object%20Reference) (OtherBodyIndex :type Integer))
  (Variables|Default|SetisIn90Box false)
  (Input|DisableInput (Game|GetPlayerController 0)))

(event OnComponentBeginOverlap(Neg90DegreesBox)
  (params (OverlappedComponent :type Primitive%20Component%20Object%20Reference) (OtherActor :type Actor%20Object%20Reference) (OtherComp :type Primitive%20Component%20Object%20Reference) (OtherBodyIndex :type Integer) (bFromSweep :type Boolean) (SweepResult :type Hit%20Result%20Structure%20%28by%20ref%29))
  (Utilities|FlowControl|Delay 0.2)
  (Variables|Default|SetisInNeg90Box true)
  (Input|EnableInput (Game|GetPlayerController 0)))

(event OnComponentEndOverlap(Neg90DegreesBox)
  (params (OverlappedComponent :type Primitive%20Component%20Object%20Reference) (OtherActor :type Actor%20Object%20Reference) (OtherComp :type Primitive%20Component%20Object%20Reference) (OtherBodyIndex :type Integer))
  (Variables|Default|SetisInNeg90Box false)
  (Input|DisableInput (Game|GetPlayerController 0)))

(event EventBeginPlay)

(event Collision|EventActorBeginOverlap
  (params (OtherActor :type Actor%20Object%20Reference)))

(event EventTick
  (params (DeltaSeconds :type Float%20%28single-precision%29)))

(event Input|KeyboardEvents|F
  (params (Key :type Key%20Structure :default "None"))
  (bind _sm_door (Variables|Default|GetSM_Door))
  (bind _returnvalue (Transformation|GetWorldRotation _sm_door))
  (:Pressed
    (Utilities|FlowControl|Sequence
      (:then_0
        (if (Variables|Default|GetisIn90Box)
          (if (or (== (.yaw _returnvalue) 9e+01) (== (.yaw _returnvalue) 0.0))
            (Utilities|FlowControl|FlipFlop
              (:A
                (bind _door_rot (Timeline|Door%20Speed%2090 Play)
                  (:Update
                    (Transformation|SetRelativeRotation _sm_door (Math|Rotator|MakeRotator 0.0 0.0 _door_rot) false false))))
              (:B
                (Timeline|Door%20Speed%2090 Reverse)))
            (else
              (bind _door_rot_2 (Timeline|Door%20Speed%20Neg%2090 Reverse)
                (:Update
                  (Transformation|SetRelativeRotation _sm_door (Math|Rotator|MakeRotator 0.0 0.0 _door_rot_2) false false)))))))
      (:then_1
        (if (Variables|Default|GetisInNeg90Box)
          (if (or (== (.yaw _returnvalue) -9e+01) (== (.yaw _returnvalue) -0.0))
            (Utilities|FlowControl|FlipFlop
              (:A
                (Timeline|Door%20Speed%20Neg%2090 Play))
              (:B
                (Timeline|Door%20Speed%20Neg%2090 Reverse)))
            (else
              (Timeline|Door%20Speed%2090 Reverse))))))))

(fn ConstructionScript)