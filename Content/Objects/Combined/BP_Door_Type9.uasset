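; A hinged door Blueprint that the first-person player toggles with the F key and that opens automatically for an AI.
; A Box overlap enables or disables input for the player, and a FlipFlop plays or reverses the DoorSpeed timeline.
; The actor referenced by TestAI drives a separate Timeline, opening on overlap and closing on exit.
; Both timelines set the door mesh's relative yaw.
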(event OnComponentBeginOverlap(Box)
  (params (OverlappedComponent :type Primitive%20Component%20Object%20Reference) (OtherActor :type Actor%20Object%20Reference) (OtherComp :type Primitive%20Component%20Object%20Reference) (OtherBodyIndex :type Integer) (bFromSweep :type Boolean) (SweepResult :type Hit%20Result%20Structure%20%28by%20ref%29))
  (if (== OtherActor (Variables|Default|GetAs%20BP%20First%20Person%20Character))
    (Input|EnableInput (Game|GetPlayerController 0))
    (elif (== OtherActor (Variables|Default|GettestAI))
      (bind _door_rot (Timeline|Timeline Play)
        (:Update
          (Transformation|SetRelativeRotation (Variables|Default|GetSM_Door) (Math|Rotator|MakeRotator 0.0 0.0 _door_rot) false false))))))

(event OnComponentEndOverlap(Box)
  (params (OverlappedComponent :type Primitive%20Component%20Object%20Reference) (OtherActor :type Actor%20Object%20Reference) (OtherComp :type Primitive%20Component%20Object%20Reference) (OtherBodyIndex :type Integer))
  (if (== (Variables|Default|GetAs%20BP%20First%20Person%20Character) OtherActor)
    (Input|DisableInput (Game|GetPlayerController 0))
    (elif (== (Variables|Default|GettestAI) OtherActor)
      (bind _door_rot (Timeline|Timeline Reverse)
        (:Update
          (Transformation|SetRelativeRotation (Variables|Default|GetSM_Door) (Math|Rotator|MakeRotator 0.0 0.0 _door_rot) false false))))))

(event EventBeginPlay
  (bind _asbp_first_person_character (Utilities|Casting|CastToBP_FirstPersonCharacter (Game|GetPlayerCharacter 0)))
  (Variables|Default|SetAs%20BP%20First%20Person%20Character _asbp_first_person_character))

(event Input|KeyboardEvents|F
  (params (Key :type Key%20Structure))
  (:Pressed
    (Utilities|FlowControl|FlipFlop
      (:A
        (bind _door_rot (Timeline|Door%20Speed Play)
          (:Update
            (Transformation|SetRelativeRotation (Variables|Default|GetSM_Door) (Math|Rotator|MakeRotator 0.0 0.0 _door_rot) false false))))
      (:B
        (Timeline|Door%20Speed Reverse)))))

(fn ConstructionScript)