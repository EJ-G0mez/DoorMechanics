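; BP_Patrol_Route_Test is a test patrol route that holds a spline of points, presumably for enemy AI to walk.
; IncrementPatrolRoute steps PatrolIndex by Direction and flips Direction at the first and last spline points, giving a back-and-forth path.
; GetSplinePointasWorldPosition returns the current point's location, though it reads it in Local space despite the name.
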(event Custom|IncrementPatrolRoute
  (bind _output_get (Variables|Default|SetpatrolIndex (+ (Variables|Default|GetpatrolIndex) (Variables|Default|Getdirection))))
  (if (== _output_get (- (Spline|GetNumberOfSplinePoints (Variables|Default|GetpatrolRoute)) 1))
    (Variables|Default|Setdirection -1)
    (elif (== (Variables|Default|GetpatrolIndex) 0)
      (Variables|Default|Setdirection 1))))

(event EventBeginPlay)

(event Collision|EventActorBeginOverlap
  (params (OtherActor :type Actor%20Object%20Reference)))

(event EventTick
  (params (DeltaSeconds :type Float%20%28single-precision%29)))

(fn ConstructionScript)

(fn GetSplinePointasWorldPosition
  (return (Spline|GetLocationatSplinePoint (Variables|Default|GetpatrolRoute) (Variables|Default|GetpatrolIndex) "Local")))